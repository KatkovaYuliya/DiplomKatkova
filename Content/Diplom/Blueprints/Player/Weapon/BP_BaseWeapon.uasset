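; Base hitscan weapon for the player, handling firing, reloading, crate ammo pickup and HUD ammo updates.
; Firing plays montages, spends ammo, traces with random spread and damages enemies, with critical damage on head-bone hits.
; Traces start at the camera, re-tracing from the muzzle when the target lies behind it, and feed a Niagara tracer.
; A fire-rate delay gates shots and loops one weapon type until IsStorFire or an empty magazine stops it.
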(event Custom|WeaponFire
  (bind _hitresult (Variables|Default|GetHitResult))
  (if (not (Variables|/Game/Diplom/Blueprints/Player/BP_Player.BP_Player_C|GetIsStorFire (Variables|Default|GetPlayerRef))) :!label _label
    (Variables|FireWeapon|SetCanFire false)
    (Animation|Montage|PlayMontage (Variables|/Script/Engine.Character|GetMesh (Variables|Default|GetPlayerRef)) (Variables|AnimMontage|GetFireAnim)
      (:then
        (Animation|Montage|PlayMontage (Variables|Default|GetWeaponMesh) (Variables|AnimMontage|GetFireWeaponAnim)
          (:then
            (CallFunction|UpdateAmmoMagazine)
            (Default|UpdateAmmoInfo (Variables|Ui|GetWeaponWidgetRef) (Variables|Ammo|GetAmmoMagazine) (Variables|Ammo|GetCurrentAmmo))
            (bind _hitresult_2 (CallFunction|LineTraceLogic))
            (CallFunction|TraceandPoint _hitresult_2)
            (CallFunction|TraceFX)
            ;[0.7232 1 0.1866] Урон по врагу. Критический урон при попадании в голову
            (bind _asbp_base_enemy (Utilities|Casting|CastToBP_BaseEnemy (.hitactor _hitresult))
              (:then
                (Game|Damage|ApplyDamage _asbp_base_enemy (Math|Float|SelectFloat (Variables|Default|GetCriticalDamage) (Variables|Default|GetDamage) (== (.hitbonename _hitresult) "head")) 0 self)
                (Effects|SpawnEmitteratLocation "/Game/Realistic_Starter_VFX_Pack_Vol2/Particles/Blood/P_Blood_Splat_Cone.P_Blood_Splat_Cone" (.location _hitresult) "0, 0, 0" "1.000000,1.000000,1.000000" false))
              (:CastFailed
                _))
            (Utilities|FlowControl|Delay (Variables|FireWeapon|GetFireRate))
            (if (Variables|Default|GetMagazineEmpty)
              (Variables|FireWeapon|SetCanFire false)
              (Development|PrintString "Кончились патроны")
              (Audio|PlaySound2D "/Engine/VREditor/Sounds/UI/Click_on_Button.Click_on_Button" 1.0 1.0 0.0 0 0)
              (else
                (Variables|FireWeapon|SetCanFire true)
                (if (Utilities|Enum|Equal(Enum) (Variables|Default|GetWeaponType) "NewEnumerator1")
                  (goto _label))))))))))

(event Custom|WeaponReload
  (if (and (CallFunction|AmmoNotEmpty) (not (CallFunction|MagazineFull)))
    (Variables|Default|SetIsReload true)
    (CallFunction|CalculateAmmo)
    (Variables|Default|SetMagazineEmpty false)
    (Default|UpdateAmmoInfo (Variables|Ui|GetWeaponWidgetRef) (Variables|Ammo|GetAmmoMagazine) (Variables|Ammo|GetCurrentAmmo))
    (Animation|Montage|PlayMontage (Variables|/Script/Engine.Character|GetMesh (Variables|Default|GetPlayerRef)) (Variables|AnimMontage|GetReloadAnim)
      (:OnCompleted
        (Variables|Default|SetIsReload false)
        (Variables|FireWeapon|SetCanFire true)))))

(event Custom|Crate
  (Variables|Ammo|SetAmmoMagazine (Variables|Ammo|GetMaxAmmoMagazine))
  (Variables|Ammo|SetCurrentAmmo (+ (Variables|Ammo|GetCurrentAmmo) 30))
  (Audio|PlaySound2D "/Game/Assets/Content/Assets/MilitaryWeapSilver/Sound/RocketLauncher/Wavs/RocketLauncher_AmmoPickup.RocketLauncher_AmmoPickup" 0.5 1.0 0.0 0 0))

(event EventBeginPlay
  (bind _asbp_player (Utilities|Casting|CastToBP_Player (Components|GetOwner)))
  (Variables|Default|SetPlayerRef _asbp_player))

(fn ConstructionScript)

(fn AttachtoHand
  (params (HandSocket :type Name))
  (Transformation|AttachComponentToComponent (Variables|/Script/Engine.Character|GetMesh (Variables|Default|GetPlayerRef)) HandSocket "SnapToTarget" "SnapToTarget" "SnapToTarget" true))

(fn SetWeaponWidgetRef
  (params (WeaponWidget :type BP%20Weapon%20Object%20Reference))
  (Variables|Ui|SetWeaponWidgetRef WeaponWidget))

(fn UpdateWidgetInfo
  (Default|UpdateWeaponWidget (Variables|Ui|GetWeaponWidgetRef) (Variables|Ammo|GetAmmoMagazine) (Variables|Ammo|GetCurrentAmmo) (Variables|Ui|GetImageHud)))

(fn UpdateAmmoMagazine
  (bind _result (Math|Integer|DecrementInt (Variables|Ammo|GetAmmoMagazine))
    (:%20%20
      (if (== _result 0)
        (Variables|Default|SetMagazineEmpty true)))))

(fn LineTraceLogic
  (bind _returnvalue (Game|GetPlayerController 0))
  (bind _weaponmesh (Variables|Default|GetWeaponMesh))
  (bind _returnvalue_2 (Transformation|GetSocketLocation _weaponmesh "MuzzleFlash"))
  (bind (_location _rotation) (Pawn|GetPlayerViewPoint _returnvalue))
  (bind (_outhit _returnvalue_3) (Collision|LineTraceByChannel _location (Math|Random|RandomPointinBoundingBox (+ _location (* (Math|Rotator|GetRotationXVector _rotation) (Variables|FireWeapon|GetFireDistance))) (* "1.000000,1.000000,1.000000" (Variables|FireWeapon|GetSpread))) "TraceTypeQuery1" false 0 "None"))
  (if _returnvalue_3
    _
    (else
      _))
  (Variables|Default|SetHitResult _outhit)
  (if (> (Class|KismetMathLibrary|DegAcos (Math|Vector|DotProduct (Math|Vector|GetForwardVector (Transformation|GetSocketRotation (Variables|Default|GetWeaponMesh) "MuzzleFlash")) (- (Math|Vector|SelectVector (.ImpactPoint (Collision|BreakHitResult _outhit)) (.TraceEnd (Collision|BreakHitResult _outhit)) (.bBlockingHit (Collision|BreakHitResult _outhit))) (Transformation|GetSocketLocation (Variables|Default|GetWeaponMesh) "MuzzleFlash")))) 9e+01)
    (bind _outhit_2 (Collision|LineTraceByChannel _returnvalue_2 (Math|Random|RandomPointinBoundingBox (+ _returnvalue_2 (* (Math|Vector|GetForwardVector (Transformation|GetSocketRotation (Variables|Default|GetWeaponMesh) "MuzzleFlash")) (Variables|FireWeapon|GetFireDistance))) (* "1.000000,1.000000,1.000000" (Variables|FireWeapon|GetSpread))) "TraceTypeQuery1" false 0 "None"))
    (bind _output_get (Variables|Default|SetHitResult _outhit_2))
    (return _output_get)
    (else
      (return (Variables|Default|GetHitResult)))))

(fn TraceandPoint
  (params (HitResult :type Hit%20Result%20Structure))
  (bind (_bblockinghit _binitialoverlap _time _distance _location _impactpoint _normal _impactnormal _physmat _hitactor _hitcomponent _hitbonename _bonename _hititem _elementindex _faceindex _tracestart _traceend) (Collision|BreakHitResult HitResult))
  (if _bblockinghit
    (Variables|Default|SetEndLineTrace _impactpoint)
    (else
      (Variables|Default|SetEndLineTrace _traceend))))

(fn TraceFX
  (bind _returnvalue (Niagara|SpawnSystematLocation (Variables|Default|GetTraceFXSystem) (Transformation|GetSocketLocation (Variables|Default|GetWeaponMesh) "MuzzleFlash")))
  (Niagara|SetNiagaraVariable(Vector3) _returnvalue "TraceTarget" (Variables|Default|GetEndLineTrace)))

(fn AmmoNotEmpty
  (return (> (Variables|Ammo|GetCurrentAmmo) 0)))

(fn MagazineFull
  (return (== (Variables|Ammo|GetAmmoMagazine) (Variables|Ammo|GetMaxAmmoMagazine))))

(fn CalculateAmmo
  (if (< (Variables|Ammo|GetCurrentAmmo) (- (Variables|Ammo|GetMaxAmmoMagazine) (Variables|Ammo|GetAmmoMagazine)))
    (Variables|Ammo|SetAmmoMagazine (+ (Variables|Ammo|GetAmmoMagazine) (Variables|Ammo|GetCurrentAmmo)))
    (Variables|Ammo|SetCurrentAmmo 0)
    (else
      (bind _output_get (LocalVariables|SetAddMagazineAmmo (- (Variables|Ammo|GetMaxAmmoMagazine) (Variables|Ammo|GetAmmoMagazine))))
      (Variables|Ammo|SetCurrentAmmo (- (Variables|Ammo|GetCurrentAmmo) _output_get))
      (Variables|Ammo|SetAmmoMagazine (+ (Variables|Ammo|GetAmmoMagazine) (LocalVariables|GetAddMagazineAmmo))))))