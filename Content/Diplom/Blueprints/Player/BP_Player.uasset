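; Player character Blueprint handling movement, sprint, walk, aiming, two-weapon combat, item pickup, health and a toggleable radio.
; BeginPlay spawns a holstered rifle and in-hand pistol; equip montages drive switching, updating the AnimBP and weapon widget.
; A looping camera line trace caches the actor Interacte picks up.
; AnyDamage drives a local Health variable, separate from BPHealth, with timer regeneration, HUD blood overlay and a montage death with screen switch.
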(event Custom|PlayerDeath
  ;[0.908 1 0.3269] Логика смерти
  (Variables|Default|SetIsDead? true)
  (Animation|Montage|PlayMontage (Variables|Character|GetMesh) "/Game/AnimStarterPack/PlayerDeath.PlayerDeath"
    (:then
      (Variables|/Script/Engine.PlayerController|SetbShowMouseCursor (Game|GetPlayerController 0) true)
      (Pawn|Components|CharacterMovement|DisableMovement (Variables|Character|GetCharacterMovement))
      (Default|SwitchScreen (Variables|/Game/Diplom/Blueprints/Player/UI/BP_Player_HUD.BP_Player_HUD_C|GetMainWidgetRef (Variables|Default|GetPlayerHUDRef))))))

(event Custom|HealRegenTimer
  ;[0.7222 0.3846 1] Регенерация здоровья
  (bind _returnvalue (Utilities|Time|SetTimerbyEvent (delegate Custom|RegenerateHealth) 5.0 true))
  (Variables|Default|SetTimerRef _returnvalue))

(event Custom|RegenerateHealth
  ;[0.7222 0.3846 1] Регенерация здоровья
  (if (== (Variables|Default|Gethealth) 1e+02)
    (Utilities|Time|ClearandInvalidateTimerbyHandle (Variables|Default|GetTimerRef))
    (else
      (bind _output_get (Variables|Default|Sethealth (Math|Float|Clamp(Float) (+ (Variables|Default|Gethealth) 5.0) 0.0 1e+02)))
      (if (>= _output_get 5e+01)
        (Default|HideBloodEffect (Variables|/Game/Diplom/Blueprints/Player/UI/BP_Player_HUD.BP_Player_HUD_C|GetMainWidgetRef (Variables|Default|GetPlayerHUDRef)))))))

(event Custom|AddAmmoCrate
  ;[1 1 1] Поднять боеприпасы
  (Default|Crate (Variables|Default|GetCurrentWeapon)))

(event Custom|HealHealth)

(event Custom|TryPickupItem
  (params (Pick :type Actor%20Object%20Reference))
  (Class|BpItemInterface|PickupItem(Message) Pick self)
  (Variables|Default|SetHit%20Actor 0))

(event EventBeginPlay
  (bind _self self)
  (bind _self_2 self)
  (Utilities|Time|SetTimerbyFunctionName 0 "ScanItem" 0.25 true)
  (bind _asbp_player_hud (Utilities|Casting|CastToBP_Player_HUD (HUD|GetHUD (Game|GetPlayerController 0))))
  (Variables|Default|SetPlayerHUDRef _asbp_player_hud)
  (Default|HealthBarWRef (Variables|Default|GetBP_Health))
  (bind _returnvalue (Game|SpawnActorfromClass "/Game/Diplom/Blueprints/Player/Weapon/BP_Pistol.BP_Pistol_C" (Transformation|GetActorTransform) "Undefined" _self_2 _self_2))
  (Variables|/Game/Diplom/Blueprints/Player/Weapon/BP_BaseWeapon.BP_BaseWeapon_C|SetIsAttachToHand _returnvalue true)
  (CallFunction|UpdateWeaponWidgetRef _returnvalue)
  (bind _output_get (Variables|Default|SetCurrentWeapon _returnvalue))
  (Utilities|Array|Add (Variables|Default|GetWeaponSlots) _output_get)
  (Transformation|AttachComponentToComponent (Variables|Default|GetCurrentWeapon) (Variables|Character|GetMesh) (Variables|/Game/Diplom/Blueprints/Player/Weapon/BP_BaseWeapon.BP_BaseWeapon_C|GetWeaponHandSocket (Variables|Default|GetCurrentWeapon)) "SnapToTarget" "SnapToTarget" "SnapToTarget" true)
  (bind _returnvalue_2 (Game|SpawnActorfromClass "/Game/Diplom/Blueprints/Player/Weapon/BP_Rifle.BP_Rifle_C" (Transformation|GetActorTransform) "Undefined" _self _self))
  (Utilities|Array|Add (Variables|Default|GetWeaponSlots) _returnvalue_2)
  (CallFunction|UpdateWeaponWidgetRef _returnvalue_2)
  (Transformation|AttachComponentToComponent _returnvalue_2 (Variables|Character|GetMesh) (Variables|/Game/Diplom/Blueprints/Player/Weapon/BP_BaseWeapon.BP_BaseWeapon_C|GetHolsterSocket _returnvalue_2) "SnapToTarget" "SnapToTarget" "SnapToTarget" true)
  (|RefAnimBP))

(event EventTick
  (params (DeltaSeconds :type Float%20%28single-precision%29))
  (if (== (Math|Vector|VectorLength (Transformation|GetVelocity)) 0.0)
    (CallFunction|MoveDirection)
    (Default|MoveDirection (Variables|Default|GetAnimBPRef) (Variables|Default|GetDirection))
    (if (Variables|Default|GetOnAim)
      (Variables|/Script/Engine.SpringArmComponent|SetTargetArmLength (Variables|Default|GetSpringArm) (Math|Float|Lerp (Variables|/Script/Engine.SpringArmComponent|GetTargetArmLength (Variables|Default|GetSpringArm)) 1e+01 0.1))
      (else
        (Variables|/Script/Engine.SpringArmComponent|SetTargetArmLength (Variables|Default|GetSpringArm) (Math|Float|Lerp (Variables|/Script/Engine.SpringArmComponent|GetTargetArmLength (Variables|Default|GetSpringArm)) 3e+02 0.1))))
    (else
      (Default|MoveDirection (Variables|Default|GetAnimBPRef) 0.0))))

(event Game|Damage|EventAnyDamage
  (params (Damage :type Float%20%28single-precision%29) (DamageType :type Damage%20Type%20Object%20Reference) (InstigatedBy :type Controller%20Object%20Reference) (DamageCauser :type Actor%20Object%20Reference))
  (bind _playerhudref (Variables|Default|GetPlayerHUDRef))
  ;[0.2116 1 0.4298] Нанесение урона игроку
  (if (not (Variables|Default|GetIsDead?))
    (bind _output_get (Variables|Default|Sethealth (- (Variables|Default|Gethealth) Damage)))
    (if (<= _output_get 0.0)
      (CallFunction|PlayerDeath)
      (else
        (if (<= (Variables|Default|Gethealth) 9e+01)
          (CallFunction|HealRegenTimer))
        (if (<= (Variables|Default|Gethealth) 5e+01)
          (Default|ShowBloodOverlap (Variables|/Game/Diplom/Blueprints/Player/UI/BP_Player_HUD.BP_Player_HUD_C|GetMainWidgetRef _playerhudref))
          (else
            (Default|HideBloodEffect (Variables|/Game/Diplom/Blueprints/Player/UI/BP_Player_HUD.BP_Player_HUD_C|GetMainWidgetRef _playerhudref))))))))

(event EventOnDeath
  (Collision|SetCollisionEnabled (Variables|Collision|GetCapsuleComponent) "NoCollision")
  (Collision|SetCollisionProfileName (Variables|Character|GetMesh) "Ragdoll" true :!class /Script/Engine.PrimitiveComponent)
  (Class|SkeletalMeshComponent|SetAllBodiesSimulatePhysics (Variables|Character|GetMesh) true)
  (Development|PrintString (Utilities|String|ToString(Float) (Variables|/Game/Diplom/Blueprints/Components/BP_Health.BP_Health_C|GetMaxHeath (Variables|Default|GetBP_Health)))))

(event Input|ActionEvents|InputActionPistolSlot
  (params (Key :type Key%20Structure :default "None"))
  ;[0.3412 1 0.619] Переключение оружия
  (:Pressed
    (if (not (Variables|/Game/Diplom/Blueprints/Player/Weapon/BP_BaseWeapon.BP_BaseWeapon_C|GetIsReload (Variables|Default|GetCurrentWeapon)))
      (if (not (Variables|/Game/Diplom/Blueprints/Player/Weapon/BP_BaseWeapon.BP_BaseWeapon_C|GetIsAttachToHand (Utilities|Array|Get(acopy) (Variables|Default|GetWeaponSlots))))
        (Variables|Default|SetIsChangeWeapon true)
        (Animation|Montage|PlayMontage (Variables|Character|GetMesh) "/Game/Diplom/Blueprints/Player/Animation/AnimMontage/AnimMontageEquipRiffleUN.AnimMontageEquipRiffleUN"
          (:OnBlendOut
            (Variables|/Game/Diplom/Blueprints/Player/Weapon/BP_BaseWeapon.BP_BaseWeapon_C|SetIsAttachToHand (Variables|Default|GetCurrentWeapon) false)
            (Animation|Montage|PlayMontage (Variables|Character|GetMesh) "/Game/Diplom/Blueprints/Player/Animation/AnimMontage/AnimMontageEcipPistol.AnimMontageEcipPistol"
              (:then
                (bind _output_get (Variables|Default|SetCurrentWeapon (Utilities|Array|Get(acopy) (Variables|Default|GetWeaponSlots))))
                (Variables|/Game/Diplom/Blueprints/Player/Weapon/BP_BaseWeapon.BP_BaseWeapon_C|SetIsAttachToHand _output_get true)
                (Default|SwitchWeaponType (Variables|Default|GetAnimBPRef) (Variables|/Game/Diplom/Blueprints/Player/Weapon/BP_BaseWeapon.BP_BaseWeapon_C|GetWeaponType (Variables|Default|GetCurrentWeapon)))
                (CallFunction|UpdateWeaponWidgetInfo))
              (:OnCompleted
                (Variables|Default|SetIsChangeWeapon false)))))))))

(event Input|ActionEvents|InputActionRifleSlot
  (params (Key :type Key%20Structure :default "None"))
  ;[0.3412 1 0.619] Переключение оружия
  (:Pressed
    (if (not (Variables|/Game/Diplom/Blueprints/Player/Weapon/BP_BaseWeapon.BP_BaseWeapon_C|GetIsReload (Variables|Default|GetCurrentWeapon)))
      (if (not (Variables|/Game/Diplom/Blueprints/Player/Weapon/BP_BaseWeapon.BP_BaseWeapon_C|GetIsAttachToHand (Utilities|Array|Get(acopy) (Variables|Default|GetWeaponSlots) 1)))
        (Variables|Default|SetIsChangeWeapon true)
        (Animation|Montage|PlayMontage (Variables|Character|GetMesh) "/Game/Diplom/Blueprints/Player/Animation/AnimMontage/AnimMontageEcipPistolUn.AnimMontageEcipPistolUn"
          (:OnBlendOut
            (Variables|/Game/Diplom/Blueprints/Player/Weapon/BP_BaseWeapon.BP_BaseWeapon_C|SetIsAttachToHand (Variables|Default|GetCurrentWeapon) false)
            (Animation|Montage|PlayMontage (Variables|Character|GetMesh) "/Game/Diplom/Blueprints/Player/Animation/AnimMontage/AnimMontageEquipRiffle.AnimMontageEquipRiffle"
              (:then
                (bind _output_get (Variables|Default|SetCurrentWeapon (Utilities|Array|Get(acopy) (Variables|Default|GetWeaponSlots) 1)))
                (Variables|/Game/Diplom/Blueprints/Player/Weapon/BP_BaseWeapon.BP_BaseWeapon_C|SetIsAttachToHand _output_get true)
                (Default|SwitchWeaponType (Variables|Default|GetAnimBPRef) (Variables|/Game/Diplom/Blueprints/Player/Weapon/BP_BaseWeapon.BP_BaseWeapon_C|GetWeaponType (Variables|Default|GetCurrentWeapon)))
                (CallFunction|UpdateWeaponWidgetInfo))
              (:OnCompleted
                (Variables|Default|SetIsChangeWeapon false)))))))))

(event Input|ActionEvents|InputActionWalk
  (params (Key :type Key%20Structure :default "None"))
  ;[1 0.3987 0.2686] Движение пешком
  (:Pressed
    (bind _output_get (Variables|Locomotion|SetIsWalk (not (Variables|Locomotion|GetIsWalk))))
    (if _output_get
      (Variables|Locomotion|SetIsSprint false)
      (CallFunction|UpdateMoveSpeed (Variables|Locomotion|GetWalkSpeed))
      (CallFunction|UpDateIsSprintAnimBP)
      (else
        (CallFunction|UpdateMoveSpeed (Variables|Locomotion|GetDefaultSpeed))))))

(event Input|ActionEvents|InputActionSprint
  (params (Key :type Key%20Structure :default "None"))
  ;[1 0.09369 0.1036] Спринт
  (:Pressed
    (if (CallFunction|IsSprintDirection)
      (Variables|Locomotion|SetIsSprint true)
      (Variables|Default|SetSprintButtonPressed true)
      (if (!= (Math|Vector|VectorLength (Transformation|GetVelocity)) 0.0)
        (Variables|Locomotion|SetIsWalk false)
        (Variables|Default|SetOnAim false)
        (CallFunction|UpdateMoveSpeed (Variables|Locomotion|GetSprintSpeed))
        (CallFunction|UpDateIsSprintAnimBP))))
  (:Released
    (bind _output_get (Variables|Locomotion|SetIsSprint false))
    (Variables|Default|SetSprintButtonPressed false)
    (if (Math|Boolean|ORBoolean _output_get (not (Variables|Locomotion|GetIsWalk)) (not (Variables|Default|GetOnAim)))
      (CallFunction|UpdateMoveSpeed (Variables|Locomotion|GetDefaultSpeed))
      (CallFunction|UpDateIsSprintAnimBP))))

(event Input|ActionEvents|InputActionJump
  (params (Key :type Key%20Structure :default "None"))
  ;[0.4436 0.5193 1] Прыжок
  (:Pressed
    (Character|Jump)))

(event Input|ActionEvents|InputActionFire
  (params (Key :type Key%20Structure :default "None"))
  (:Pressed
    (if (not (Variables|Locomotion|GetIsSprint))
      (Variables|Default|SetIsStorFire false)
      (if (and (not (Variables|Default|GetIsChangeWeapon)) (Variables|/Game/Diplom/Blueprints/Player/Weapon/BP_BaseWeapon.BP_BaseWeapon_C|GetCanFire (Variables|Default|GetCurrentWeapon)))
        (Default|WeaponFire (Variables|Default|GetCurrentWeapon)))))
  (:Released
    (Variables|Default|SetIsStorFire true)))

(event Input|ActionEvents|InputActionReload
  (params (Key :type Key%20Structure :default "None"))
  ;[0.08731 0.4212 1] Перезарядка оружия
  (:Pressed
    (Default|WeaponReload (Variables|Default|GetCurrentWeapon))))

(event Input|ActionEvents|InputActionAim
  (params (Key :type Key%20Structure :default "None"))
  ;[1 1 1] Прицеливание
  (:Pressed
    (Variables|Default|SetOnAim true)
    (Variables|Locomotion|SetIsSprint false)
    (CallFunction|UpdateMoveSpeed (Variables|Locomotion|GetDefaultSpeed))
    (CallFunction|UpDateIsSprintAnimBP))
  (:Released
    (Variables|Default|SetOnAim false)
    (if (Variables|Default|GetSprintButtonPressed)
      (Variables|Locomotion|SetIsSprint true)
      (CallFunction|UpdateMoveSpeed (Variables|Locomotion|GetSprintSpeed))
      (CallFunction|UpDateIsSprintAnimBP)
      (if (Variables|Default|GetSprintButtonPressed)
        _))))

(event Input|ActionEvents|InputActionRadio
  (params (Key :type Key%20Structure :default "None"))
  ;[1 0.3202 0.2104] Play Radio
  (:Pressed
    (if (Variables|Default|GetIsPlayingSound)
      (Variables|Default|SetIsPlayingSound false)
      (Audio|Components|Audio|Stop (Variables|Default|GetStopSound))
      (Default|StopPlayRadio (Variables|/Game/Diplom/Blueprints/Player/UI/BP_Player_HUD.BP_Player_HUD_C|GetMainWidgetRef (Variables|Default|GetPlayerHUDRef)))
      (else
        (Variables|Default|SetIsPlayingSound true)
        (bind _returnvalue (Audio|SpawnSound2D (Variables|Default|GetSound) 1.0 1.0 0.0 0))
        (Variables|Default|SetStopSound _returnvalue)
        (Default|PlayRadio (Variables|/Game/Diplom/Blueprints/Player/UI/BP_Player_HUD.BP_Player_HUD_C|GetMainWidgetRef (Variables|Default|GetPlayerHUDRef)))))))

(event Input|ActionEvents|InputActionInteracte
  (params (Key :type Key%20Structure :default "None"))
  (:Pressed
    (bind _hit_actor (Variables|Default|GetHit%20Actor)
      (:then
        (CallFunction|TryPickupItem _hit_actor))
      (:else))))

(event Input|AxisEvents|InputAxisMoveForward
  (params (AxisValue :type Float%20%28single-precision%29))
  ;[0.9567 1 0.7098] Передвижение персонажа
  (Pawn|Input|AddMovementInput (Transformation|GetActorForwardVector) AxisValue false))

(event Input|AxisEvents|InputAxisMoveRight
  (params (AxisValue :type Float%20%28single-precision%29))
  ;[0.9567 1 0.7098] Передвижение персонажа
  (Pawn|Input|AddMovementInput (Transformation|GetActorRightVector) AxisValue false)
  (if (!= AxisValue 0.0)
    (CallFunction|BrealSprint)))

(event Input|AxisEvents|InputAxisTurn
  (params (AxisValue :type Float%20%28single-precision%29))
  ;[1 0.9769 0.6244] Управление камерой
  (Pawn|Input|AddControllerYawInput AxisValue))

(event Input|AxisEvents|InputAxisLookUp
  (params (AxisValue :type Float%20%28single-precision%29))
  ;[1 0.9769 0.6244] Управление камерой
  (Pawn|Input|AddControllerPitchInput AxisValue))

(event Input|KeyboardEvents|H
  (params (Key :type Key%20Structure :default "None"))
  (:Pressed
    (Default|Heal (Variables|Default|GetBP_Health) 3.0)
    (Development|PrintString (Utilities|String|ToString(Float) (Variables|/Game/Diplom/Blueprints/Components/BP_Health.BP_Health_C|GetCurrentHealth (Variables|Default|GetBP_Health))))))

(fn ConstructionScript)

(fn MoveDirection
  (bind _returnvalue (Transformation|GetVelocity))
  (bind _returnvalue_2 (Transformation|GetActorForwardVector))
  (bind _returnvalue_3 (Math|Vector|Normalize _returnvalue))
  (Variables|Default|SetDirection (* (Class|KismetMathLibrary|DegAcos (Math|Vector|DotProduct _returnvalue_3 _returnvalue_2)) (Math|Float|Sign(Float) (.z (Math|Vector|CrossProduct _returnvalue_3 _returnvalue_2))))))

(fn UpdateMoveSpeed
  (params (Speed :type Float%20%28double-precision%29))
  (Variables|/Script/Engine.CharacterMovementComponent|SetMaxWalkSpeed (Variables|Character|GetCharacterMovement) Speed))

(fn UpDateIsSprintAnimBP
  (Default|ActivateSprint (Variables|Default|GetAnimBPRef) (Variables|Locomotion|GetIsSprint)))

(fn IsSprintDirection
  (return (and (<= (Variables|Default|GetDirection) 3e+01) (>= (Variables|Default|GetDirection) -3e+01))))

(fn BrealSprint
  (Variables|Locomotion|SetIsSprint false)
  (CallFunction|UpdateMoveSpeed (Variables|Locomotion|GetDefaultSpeed))
  (CallFunction|UpDateIsSprintAnimBP))

(fn UpdateWeaponWidgetRef
  (params (Weapon :type BP%20Base%20Weapon%20Object%20Reference))
  (Default|SetWeaponWidgetRef Weapon (Variables|/Game/Diplom/Blueprints/Player/UI/BP_Player_HUD.BP_Player_HUD_C|GetWeaponWidgetRef (Variables|Default|GetPlayerHUDRef))))

(fn UpdateWeaponWidgetInfo
  (Default|UpdateWidgetInfo (Variables|Default|GetCurrentWeapon)))

(fn ScanItem
  (bind _camera (Variables|Default|GetCamera))
  (bind _returnvalue (Transformation|GetWorldLocation _camera))
  (bind (_outhit _returnvalue_2) (Collision|LineTraceByChannel _returnvalue (+ _returnvalue (* (Math|Vector|GetForwardVector (Transformation|GetWorldRotation _camera)) 5e+02)) "TraceTypeQuery1" false 0 "None"))
  (if _returnvalue_2
    (Variables|Default|SetHit%20Actor (.HitActor (Collision|BreakHitResult _outhit)))))

(fn AddItemtoInvent)

(fn IsPlayer
  (return true))

(fn RefPlayer
  (return self))