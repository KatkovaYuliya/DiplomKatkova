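; BP_Health is a health component that tracks its owner's current health against a maximum, starting full on BeginPlay.
; TakeDamage subtracts damage and, at zero or below, sets health to zero and sends OnDeathMessage to the owner.
; Heal adds health up to the maximum, never lowering it.
; HealthBarWRef caches the player HUD's health bar through an owner message, but the widget update calls are disconnected.
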(event Custom|Take%20Damage
  (params (Damage :type Float%20%28double-precision%29))
  ;[1 1 1] Получение урона
  (if (<= (- (Variables|Default|GetCurrentHealth) Damage) 0.0)
    (Variables|Default|SetCurrentHealth 0.0)
    (Class|HelperHealthComponent|OnDeath(Message) (Components|GetOwner))
    (else
      (bind _output_get (Variables|Default|SetCurrentHealth (- (Variables|Default|GetCurrentHealth) Damage))))))

(event Custom|Heal
  (params (Amount :type Float%20%28double-precision%29))
  ;[1 1 1] Лечение
  (Variables|Default|SetCurrentHealth (Math|Float|Clamp(Float) (+ Amount (Variables|Default|GetCurrentHealth)) (Variables|Default|GetCurrentHealth) (Variables|Default|GetMaxHeath))))

(event EventBeginPlay
  (Variables|Default|SetCurrentHealth (Variables|Default|GetMaxHeath)))

(event EventHealthBarWRef
  (bind _player (Class|HelperHealthComponent|RefPlayer(Message) (Components|GetOwner)))
  (Variables|Default|SetHealthBarWidgetRef (Variables|/Game/Diplom/Blueprints/Player/UI/BP_Player_HUD.BP_Player_HUD_C|GetBP%20Widget%20Health%20Bar (Variables|/Game/Diplom/Blueprints/Player/BP_Player.BP_Player_C|GetPlayerHUDRef _player))))

(fn RefPlayer
  (return 0))